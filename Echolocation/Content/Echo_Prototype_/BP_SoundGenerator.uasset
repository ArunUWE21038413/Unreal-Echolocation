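; Short-lived sound source actor that visualizes a sound as an expanding ripple from its location, using post-process and decal materials.
; Creates dynamic instances of both materials and adds the post-process one to the PostProcessVolume found in the level.
; A timeline grows their shared radius to SoundRange and animates intensities, then destroys the decal.
; After a delay, the finish timeline's update sets intensity, removes the blendable and destroys the actor.
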(event `self.ReceiveBeginPlay`
  (bind _returnvalue (* (`self.SoundRange`) 0.05))
  (bind _weightedblendables_array (break `WeightedBlendables` (break `PostProcessSettings` (`PostProcessVolume.Settings` (`self.PostProcessVolume`)))))
  (bind _returnvalue_2 (`GameplayStatics.GetActorOfClass` "/Script/Engine.PostProcessVolume"))
  (set `self.PostProcessVolume` _returnvalue_2)
  (bind _returnvalue_3 (`KismetMaterialLibrary.CreateDynamicMaterialInstance` "/Game/Echo_Prototype_/M_Post_Process_Add.M_Post_Process_Add"))
  (set `self.PostProcessMaterial` _returnvalue_3)
  (`SceneComponent.SetRelativeScale3D` (`self.Decal`) (`KismetMathLibrary.MakeVector` _returnvalue _returnvalue _returnvalue))
  (`MaterialInstanceDynamic.SetVectorParameterValue` (`self.PostProcessMaterial`) "Location" (`KismetMathLibrary.Conv_VectorToLinearColor` (`self.K2_GetActorLocation`)))
  ;[1 1 1] Add post process material to one of the post pprocess arrays
  (`KismetArrayLibrary.Array_Add` _weightedblendables_array (`KismetArrayLibrary.Array_Random` (`|MakeArray` (make `WeightedBlendable` 1.0 (`self.PostProcessMaterial`)) (make `WeightedBlendable` 1.0 (`self.PostProcessMaterial`)) (make `WeightedBlendable` 1.0 (`self.PostProcessMaterial`)) (make `WeightedBlendable` 1.0 (`self.PostProcessMaterial`)) (make `WeightedBlendable` 1.0 (`self.PostProcessMaterial`)))))
  (`self.CustomEvent_Expansion`)
  (`KismetSystemLibrary.Delay` 3.0))

(event `CustomEvent_Expansion`
  (bind (_direction _radius _intensity _decal_intensity) (`Timeline|Decal_Timeline` :!via `PlayFromStart`)
    (:`Update`
      (`self.UpdateRadius` (`KismetMathLibrary.Lerp` (`self.StartRange`) (`self.SoundRange`) _radius))
      (`MaterialInstanceDynamic.SetScalarParameterValue` (`self.PostProcessMaterial`) "Intensity" _intensity)
      (`MaterialInstanceDynamic.SetScalarParameterValue` (`self.M_Decal`) "Decal_Intensity" _decal_intensity))
    (:`Finished`
      (`ActorComponent.K2_DestroyComponent` (`self.Decal`))
      (`KismetSystemLibrary.Delay` 2.0)
      (`self.CustomEvent_Finish`))))

(event `CustomEvent_Finish`
  (bind _weightedblendables_array (break `WeightedBlendables` (break `PostProcessSettings` (`PostProcessVolume.Settings` (`self.PostProcessVolume`)))))
  (bind (_direction _intensity) (`Timeline|Finish_Timeline`)
    (:`Update`
      (`MaterialInstanceDynamic.SetScalarParameterValue` (`self.PostProcessMaterial`) "Intensity" _intensity)
      (`KismetArrayLibrary.Array_RemoveItem` _weightedblendables_array (make `WeightedBlendable` 1.0 (`self.PostProcessMaterial`)))
      (`self.K2_DestroyActor`))))

(fn `UpdateRadius`
  (params (Radius :type "Float (double-precision)"))
  (`MaterialInstanceDynamic.SetScalarParameterValue` (`self.PostProcessMaterial`) "Radius" Radius)
  (`MaterialInstanceDynamic.SetScalarParameterValue` (`self.M_Decal`) "Radius" Radius))

(fn `UserConstructionScript`
  (bind _returnvalue (`KismetMaterialLibrary.CreateDynamicMaterialInstance` "/Game/Echo_Prototype_/M_RippleDecal.M_RippleDecal"))
  (bind _output_get (set `self.M_Decal` _returnvalue))
  (`MaterialInstanceDynamic.SetVectorParameterValue` _output_get "Color" (`self.Decal_Color`))
  (`MaterialInstanceDynamic.SetVectorParameterValue` (`self.M_Decal`) "Location" (`KismetMathLibrary.Conv_VectorToLinearColor` (`self.K2_GetActorLocation`)))
  (`DecalComponent.SetDecalMaterial` (`self.Decal`) (`self.M_Decal`)))